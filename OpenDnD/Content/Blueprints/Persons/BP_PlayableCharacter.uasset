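; Playable character Blueprint that handles interaction, dialog UI and inventory toggling for the player.
; Overlap events track the current actor with an Interaction component, and the Interact input starts dialog with it.
; Dialog start and end events, bound on BeginPlay, add and remove the UI_Dialog widget.
; The Inventory input toggles UI_Inventory, switching mouse visibility through BP_PlayerController and restoring viewport focus on close.
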(event `self.ReceiveBeginPlay`
  (add `self.OnDialogStart` (delegate `On Dialog Start`))
  (add `self.OnDialogEnd` (delegate `On Dialog End`)))

(event `On Dialog Start`
  (bind _returnvalue (`|CreateWidget` "/Game/Blueprints/UI/UI_Dialog.UI_Dialog_C"))
  (`UserWidget.AddToPlayerScreen` _returnvalue 0))

(event `On Dialog End`
  (bind _foundwidgets (`WidgetBlueprintLibrary.GetAllWidgetsOfClass` "/Game/Blueprints/UI/UI_Dialog.UI_Dialog_C"))
  (`Widget.RemoveFromParent` _foundwidgets))

(event `self.ReceiveTick`
  (params (DeltaSeconds :type "Float (single-precision)")))

(event `self.ReceiveActorBeginOverlap`
  (params (OtherActor :type "Actor Object Reference"))
  (`/Engine/EditorBlueprintResources/StandardMacros.IsValid` (`self.GetComponentByClass` OtherActor "/Game/Blueprints/Components/Interaction.Interaction_C")
    (:`Is Valid`
      (set `self.InteractingActor` OtherActor)
      (`KismetSystemLibrary.PrintString` (`KismetStringLibrary.Concat_StrStr` "Adding interacting actor: " (`KismetSystemLibrary.GetDisplayName` OtherActor)) false))))

(event `self.ReceiveActorEndOverlap`
  (params (OtherActor :type "Actor Object Reference"))
  (`/Engine/EditorBlueprintResources/StandardMacros.IsValid` (`self.GetComponentByClass` OtherActor "/Game/Blueprints/Components/Interaction.Interaction_C")
    (:`Is Valid`
      (`KismetSystemLibrary.PrintString` (`KismetStringLibrary.Concat_StrStr` "Removing interacting actor: " (`KismetSystemLibrary.GetDisplayName` (`self.InteractingActor`))) false)
      (set `self.InteractingActor` null))))

(event `InputAction|Interact`
  (params (Key :type "Key Structure"))
  (:`Released`
    (`/Engine/EditorBlueprintResources/StandardMacros.IsValid` (`self.InteractingActor`)
      (:`Is Valid`
        (`self.StartDialog`)
        (`self.On Dialog Start`)))))

(event `InputAction|Inventory`
  (params (Key :type "Key Structure"))
  (:`Released`
    (bind _asbp_player_controller (cast `/Game/Blueprints/Persons/BP_PlayerController` (`self.GetController`)))
    (if (`self.IsInventoryFocused`)
      (`DPlayerController.HideMouse` _asbp_player_controller)
      (set `self.IsInventoryFocused` false)
      (`Widget.RemoveFromParent` (stale _returnvalue))
      (`WidgetBlueprintLibrary.SetFocusToGameViewport`)
      (else
        (`DPlayerController.ShowMouse` _asbp_player_controller)
        (set `self.IsInventoryFocused` true)
        (bind _returnvalue (`|CreateWidget` "/Game/Blueprints/UI/UI_Inventory.UI_Inventory_C"))
        (`UserWidget.AddToPlayerScreen` _returnvalue 0)))))

(fn `UserConstructionScript`)