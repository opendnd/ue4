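; BP_AllyCharacter is an ally character that provides quest-related dialog functions for the player conversation.
; AddQuest only prints a debug message, advances this character's dialog and ends the player's dialog.
; CheckQuest sends the player to response 1 and advances the dialog if the player's item list is non-empty, otherwise to response 2.
; Events and construction just defer to the parent class.
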(event `self.ReceiveBeginPlay`
  (`parent.ReceiveBeginPlay`))

(event `self.ReceiveActorBeginOverlap`
  (params (OtherActor :type "Actor Object Reference"))
  (`parent.ReceiveActorBeginOverlap` OtherActor))

(fn `AddQuest`
  (`KismetSystemLibrary.PrintString` "Adding the quest")
  (`self.IncrementDialog`)
  (bind _asbp_playable_character (cast `/Game/Blueprints/Persons/BP_PlayableCharacter` (`GameplayStatics.GetPlayerCharacter` 0)))
  (`DPlayableCharacter.EndDialog` _asbp_playable_character))

(fn `CheckQuest`
  (bind _asbp_playable_character (cast `/Game/Blueprints/Persons/BP_PlayableCharacter` (`GameplayStatics.GetPlayerCharacter` 0)))
  (if (> (`KismetArrayLibrary.Array_Length` (`.items` (break `DPersonStruct` (`DPersonCharacter.Person` _asbp_playable_character)))) 0)
    (`DPlayableCharacter.GoToResponse` _asbp_playable_character 1)
    (`self.IncrementDialog`)
    (else
      (`DPlayableCharacter.GoToResponse` _asbp_playable_character 2))))

(fn `UserConstructionScript`
  (`parent.UserConstructionScript`))