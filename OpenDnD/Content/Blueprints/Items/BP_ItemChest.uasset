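; Item chest Blueprint that hands its items to the player character.
; GetItems casts player 0's character to BP_PlayableCharacter, passes the Items from its Item variable to AddItems, then calls EndDialog on the character.
; The event graph holds only disabled default events, and nothing in this Blueprint calls GetItems.
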(fn `GetItems`
  (bind _asbp_playable_character (cast `/Game/Blueprints/Persons/BP_PlayableCharacter` (`GameplayStatics.GetPlayerCharacter` 0)))
  (`DPlayableCharacter.AddItems` _asbp_playable_character (`.items` (break `DItemStruct` (`self.Item`))))
  (`DPlayableCharacter.EndDialog` _asbp_playable_character))

(fn `UserConstructionScript`
  (`parent.UserConstructionScript`))