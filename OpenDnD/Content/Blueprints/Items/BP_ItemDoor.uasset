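; BP_ItemDoor is a door item that swings open and ends the player's dialog when it opens.
; BeginPlay caches the root component's relative rotation.
; OpenDoor snaps the root to a fixed yaw, keeping the cached pitch and roll, then calls EndDialog on the player's BP_PlayableCharacter.
; CloseDoor is an empty stub, and the file has no animation or overlap logic.
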(event `self.ReceiveBeginPlay`
  (`parent.ReceiveBeginPlay`)
  (set `self.OriginalRotator` (`SceneComponent.RelativeRotation` (`self.DefaultSceneRoot`))))

(fn `CloseDoor`)

(fn `OpenDoor`
  (`SceneComponent.K2_SetRelativeRotation` (`self.DefaultSceneRoot`) (`KismetMathLibrary.MakeRotator` (.roll (`self.OriginalRotator`)) (.pitch (`self.OriginalRotator`)) 120.0) false false)
  (bind _asbp_playable_character (cast `/Game/Blueprints/Persons/BP_PlayableCharacter` (`GameplayStatics.GetPlayerCharacter` 0)))
  (`DPlayableCharacter.EndDialog` _asbp_playable_character))

(fn `UserConstructionScript`
  (`parent.UserConstructionScript`))