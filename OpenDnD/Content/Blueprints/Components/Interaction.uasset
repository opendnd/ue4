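; Interaction component that lets the playable character engage its owning actor for dialog on overlap.
; On begin overlap it shows the owner's TextRender, sets the owner as InteractingActor, and passes the current dialog from a DPersonCharacter or DItem owner to the character before calling SetDialogPrompt.
; On end overlap it hides the text but sets InteractingActor to the owner again rather than clearing it.
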(event `self.ReceiveBeginPlay`
  (bind _returnvalue (`self.GetOwner`))
  (add `Actor.OnActorBeginOverlap` _returnvalue (delegate `BeginOverlap`))
  (add `Actor.OnActorEndOverlap` _returnvalue (delegate `EndOverlap`)))

(event `BeginOverlap`
  (params (OverlappedActor :type "Actor Object Reference") (OtherActor :type "Actor Object Reference"))
  (bind _returnvalue (`self.GetOwner`))
  (bind _asbp_playable_character (cast `/Game/Blueprints/Persons/BP_PlayableCharacter` OtherActor))
  (`self.SetVisibility` (`Actor.GetComponentByClass` _returnvalue "/Script/Engine.TextRenderComponent") true false)
  (set `DPlayableCharacter.InteractingActor` _returnvalue _asbp_playable_character)
  (bind _asdperson_character (cast `DPersonCharacter` _returnvalue)
    (:`then`
      (bind _returnvalue_2 (`DPersonCharacter.GetCurrentDialog` _asdperson_character))
      (set `DPlayableCharacter.Dialog` _returnvalue_2 _asbp_playable_character))
    (:`CastFailed`
      (bind _asditem (cast `DItem` _returnvalue))
      (bind _returnvalue_3 (`DItem.GetCurrentDialog` _asditem))
      (set `DPlayableCharacter.Dialog` _returnvalue_3 _asbp_playable_character)))
  (`DPlayableCharacter.SetDialogPrompt` _asbp_playable_character))

(event `EndOverlap`
  (params (OverlappedActor :type "Actor Object Reference") (OtherActor :type "Actor Object Reference"))
  (bind _returnvalue (`self.GetOwner`))
  (bind _asbp_playable_character (cast `/Game/Blueprints/Persons/BP_PlayableCharacter` OtherActor))
  (`self.SetVisibility` (`Actor.GetComponentByClass` _returnvalue "/Script/Engine.TextRenderComponent") false false)
  (set `DPlayableCharacter.InteractingActor` _returnvalue _asbp_playable_character))